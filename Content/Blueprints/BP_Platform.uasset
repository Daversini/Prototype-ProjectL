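; BP_Platform is a moving platform that travels back and forth while its linked interactable object reports light.
; On BeginPlay it stores its start location and binds to the interactable's interaction event, whose HasLight flag plays or stops a timeline.
; The timeline lerps the actor between the start location and a relative EndPosition offset, reversing on each finish to ping-pong without sweeping.
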(event Custom|OnInteraction_Event
  (params (HasLight :type Boolean))
  (bind _startposition (Variables|Default|GetStartPosition))
  (Variables|Default|SetIsMoving HasLight)
  (if (Variables|Default|GetIsMoving)
    (bind (_direction _value) (Timeline|Timeline Play)
      (:Update
        (Transformation|SetActorLocation (Math|Vector|Lerp(Vector) _startposition (+ (Variables|Default|GetEndPosition) _startposition) _value) false false))
      (:Finished
        (switch Utilities|FlowControl|Switch|SwitchonETimelineDirection _direction
          (:Forward
            (Timeline|Timeline ReverseFromEnd))
          (:Backward
            (Timeline|Timeline PlayFromStart)))))
    (else
      (Timeline|Timeline Stop))))

(event EventBeginPlay
  (Variables|Default|SetStartPosition (Transformation|GetActorLocation))
  (EventDispatchers|AssignOnInteraction (Variables|Default|GetInteractableObj) (delegate Custom|OnInteraction_Event)))

(fn ConstructionScript)